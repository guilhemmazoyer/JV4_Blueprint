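; BP_ShowCollected is an actor that displays a running count of collected pickups on a TextRender component.
; On BeginPlay it casts the player pawn to BP_ThirdPersonCharacter and binds to that character's PickupCollected event dispatcher.
; ShowCollected increments PickupAmount and writes it after BaseText, so the display updates through events without polling.
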(event EventBeginPlay
  (bind _asbp_third_person_character (Utilities|Casting|CastToBP_ThirdPersonCharacter (Game|Player|GetPlayerPawn 0)))
  (EventDispatchers|BindEventtoPickupCollected _asbp_third_person_character (EventDispatchers|CreateEvent :!event ShowCollected)))

(fn ConstructionScript)

(fn ShowCollected
  (bind _result (Math|Integer|IncrementInt (Variables|Default|GetPickupAmount))
    (:%20%20
      (Rendering|Components|TextRender|SetText (Variables|Default|GetTextRender) (Utilities|Text|ToText(String) (Utilities|String|Append (Variables|Default|GetBaseText) (Utilities|String|ToString(Integer) _result)))))))