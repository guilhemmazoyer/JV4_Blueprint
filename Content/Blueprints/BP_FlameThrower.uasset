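; Rotating flamethrower trap actor that periodically spawns a line of BP_Fire actors.
; A self-retriggering event started on BeginPlay yaws the Cube by a set angle, counting steps with a Delay between each.
; At the counter limit, it spawns evenly spaced flames outward from the Sphere along the horizontal Cube-to-Sphere direction, resets the count and waits for the flame duration.
; The flame-destroy loop and debug prints are unconnected.
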(event Custom|Trigger_FlameThrower
  (Math|Integer|IncrementInt (Variables|Default|Getcounter)
    (:%20%20
      (bind _appliedrotation (CallFunction|FRotateonAxis (Variables|Default|GetRotationAngle)))
      (Transformation|AddWorldRotation (Variables|Default|GetCube) _appliedrotation false false)
      (if (>= (Variables|Default|Getcounter) (Variables|Default|GetMaxCounterValue))
        (bind _flames (CallFunction|FDrawFireShape))
        (Utilities|FlowControl|Delay (Variables|Default|GetFlameDuration))
        (else
          (Utilities|FlowControl|Delay (Variables|Default|GetRotationSpeed))))
      (CallFunction|TriggerFlameThrower))))

(event EventBeginPlay
  (Utilities|FlowControl|Sequence
    (:then_3
      (CallFunction|TriggerFlameThrower))))

(fn ConstructionScript)

(fn FPrintCubeScale
  (Development|PrintString (Utilities|String|Append (LocalVariables|Getemphasis) (Utilities|String|ToString(Vector) (Variables|/Script/Engine.SceneComponent|GetRelativeScale3D (Variables|Default|GetCube)))) true true "(R=0.000000,G=0.660000,B=1.000000,A=1.000000)" 5.0))

(fn FPrintSphereLocation
  (Development|PrintString (Utilities|String|Append (LocalVariables|Getemphasis) (Utilities|String|ToString(Vector) (Variables|/Script/Engine.SceneComponent|GetRelativeLocation (Variables|Default|GetSphere)))) true true "(R=0.000000,G=0.660000,B=1.000000,A=1.000000)" 5.0))

(fn FRotateonAxis
  (params (rotationAngle :type Integer))
  (return (Math|Rotator|MakeRotator 0.0 0.0 (Math|Conversions|ToFloat(Integer) rotationAngle))))

(fn FDrawFireShape
  (bind _sphere (Variables|Default|GetSphere))
  (bind _returnvalue (Transformation|GetWorldLocation _sphere))
  (Utilities|Array|Clear (Variables|Default|GetFlames))
  (for _index (range 0 (Variables|Default|GetRange%20of%20Flames))
    (bind _returnvalue_2 (Game|SpawnActorfromClass "/Game/Blueprints/BP_Fire.BP_Fire_C" (Math|Conversions|ToTransform(Vector) (+ (* (* (* _index 100) (Math|Vector|GetUnitDirection(Vector) (Transformation|GetWorldLocation (Variables|Default|GetCube)) _returnvalue)) "1.000000,1.000000,0.000000") _returnvalue)) "Undefined" 0 0))
    (Utilities|Array|AppendArray (Variables|Default|GetFlames) (Utilities|Array|MakeArray _returnvalue_2)))
  (Variables|Default|Setcounter 0)
  (return (Variables|Default|GetFlames)))