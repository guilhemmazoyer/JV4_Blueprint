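; BP_EndGame is a finish-line trigger that ends the level when the third-person character enters its box.
; On overlap it compares the character's AmountCollected with PickupNeededToFinish.
; With enough pickups, it plays music and prints a win message once.
; Otherwise it spawns an explosion, destroys the character and reloads ThirdPersonMap after a short delay; a disconnected test copy of this logic remains unused.
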(event OnComponentBeginOverlap(Box)
  (params (OverlappedComponent :type Primitive%20Component%20Object%20Reference) (OtherActor :type Actor%20Object%20Reference) (OtherComp :type Primitive%20Component%20Object%20Reference) (OtherBodyIndex :type Integer) (bFromSweep :type Boolean) (SweepResult :type Hit%20Result%20Structure%20%28by%20ref%29))
  (bind _asbp_third_person_character (Utilities|Casting|CastToBP_ThirdPersonCharacter OtherActor))
  ;[1 1 1] Condition a deux résultat (if)
  (if (>= (Variables|/Game/ThirdPerson/Blueprints/BP_ThirdPersonCharacter.BP_ThirdPersonCharacter_C|GetAmountCollected _asbp_third_person_character) (Variables|Default|GetPickupNeededToFinish))
    (Utilities|FlowControl|DoOnce false
      (:Completed
        (Audio|PlaySound2D "/Game/StarterContent/Audio/Starter_Music_Cue.Starter_Music_Cue" 1.0 1.0 0.0 0 0)
        (Development|PrintString "You Win !")))
    (else
      (Effects|SpawnEmitteratLocation "/Game/StarterContent/Particles/P_Explosion.P_Explosion" (Transformation|GetWorldLocation (Variables|Default|GetBox)))
      (Actor|DestroyActor _asbp_third_person_character)
      (Development|PrintString "You loose ... Restarting ...")
      (Utilities|FlowControl|Delay 2.0)
      (Game|OpenLevel(byName) "ThirdPersonMap"))))

(event Collision|EventActorBeginOverlap
  (params (OtherActor :type Actor%20Object%20Reference))
  ;[1 1 1] Remove
)

(fn ConstructionScript)