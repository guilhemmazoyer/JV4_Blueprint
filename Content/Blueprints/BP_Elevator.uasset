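; BP_Elevator is an elevator actor whose Cube platform travels back and forth between StartPoint and EndPoint.
; On BeginPlay it sets EndPoint's relative Z from the ElevatorEndPoint variable and starts moving.
; The ElevatorMove timeline lerps the Cube's world location between the two points without sweep.
; Each finish re-triggers MoveElevator, where a FlipFlop alternates forward and reverse playback for an endless loop.
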(event Custom|MoveElevator
  ;[1 1 1] Move elevator
  (Utilities|FlowControl|FlipFlop
    (:A
      (bind _alpha (Timeline|ElevatorMove Play)
        (:Update
          (Transformation|SetWorldLocation (Variables|Default|GetCube) (Math|Vector|Lerp(Vector) (Transformation|GetWorldLocation (Variables|Default|GetStartPoint)) (Transformation|GetWorldLocation (Variables|Default|GetEndPoint)) _alpha) false false))
        (:Finished
          (CallFunction|MoveElevator))))
    (:B
      (Timeline|ElevatorMove ReverseFromEnd))))

(event EventBeginPlay
  ;[1 1 1] Event begin
  (Transformation|SetRelativeLocation (Variables|Default|GetEndPoint) (Math|Vector|MakeVector 0.0 0.0 (Variables|Default|GetElevatorEndPoint)) false false)
  (CallFunction|MoveElevator))

(fn ConstructionScript)